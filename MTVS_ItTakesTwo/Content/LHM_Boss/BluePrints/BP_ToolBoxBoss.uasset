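; Tool box boss Blueprint whose streamingCine event plays the 2Phage level sequence as a boss cutscene.
; The event sets a timer from the sequence length, disables player input and turns off its own collision.
; It then loops over gathered actors, unhiding class-matched ones and stopping their tick.
; StartCinematic and other events are empty, and the CallCutSin and StreamingCine calls sit in unreachable nodes.
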(event `self.ReceiveBeginPlay`)

(event `self.ReceiveActorBeginOverlap`
  (params (OtherActor :type "Actor Object Reference")))

(event `self.StartCinematic`)

(event `streamingCine`
  (bind (_outactor _returnvalue) (`LevelSequencePlayer.CreateLevelSequencePlayer` "/Game/LHM_Boss/LevelSequence/2Phage.2Phage"))
  (`MovieSceneSequencePlayer.Play` _returnvalue)
  (bind _returnvalue_2 (message `AnimationDataModel.GetPlayLength` _returnvalue))
  (`KismetSystemLibrary.K2_SetTimerDelegate` :`Time` _returnvalue_2)
  (`self.DisableInput` (`GameplayStatics.GetPlayerCharacter` 0) (`GameplayStatics.GetPlayerController` 0))
  (`self.SetActorEnableCollision` false)
  (bind _outactors (`GameplayStatics.GetAllActorsOfClass` null))
  (for _array_element _outactors
    (bind _returnvalue_3 (`GameplayStatics.GetObjectClass` _array_element))
    (if (or (`KismetMathLibrary.ClassIsChildOf` _returnvalue_3) (== _returnvalue_3 null))
      (`self.SetActorHiddenInGame` _array_element false)
      (`self.SetActorTickEnabled` _array_element false)))
  (cast `GameInstance` (`GameplayStatics.GetGameInstance`)))

(fn `UserConstructionScript`)