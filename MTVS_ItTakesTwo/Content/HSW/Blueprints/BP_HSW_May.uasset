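; BP_HSW_May is an actor, apparently the player's May, that spawns a BP_HSW_Hammer2 on BeginPlay and attaches it to its Scene component.
; The attack input plays a timeline that rotates Scene from its initial rotation to swing the hammer.
; The hanging input, when the hammer's CanHanging is true, calls ClickToMove and sets FixPlayer, so Tick pins the actor to the hammer's PlayerAttachingPoint socket.
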(event `self.ReceiveBeginPlay`
  (set `self.initRotate` (`SceneComponent.RelativeRotation` (`self.Scene`)))
  (bind _returnvalue (`|SpawnActorFromClass` "/Game/HSW/Blueprints/BP_HSW_Hammer2.BP_HSW_Hammer2_C" (`SceneComponent.GetRelativeTransform` (`self.Scene`)) "Undefined" "MultiplyWithRoot" null null))
  (bind _output_get (set `self.Hammer2` _returnvalue))
  (`self.K2_AttachToComponent` _output_get (`self.Scene`) "None" "KeepRelative" "KeepRelative" "KeepRelative" true))

(event `self.ReceiveTick`
  (params (DeltaSeconds :type "Float (single-precision)"))
  (if (`self.bFixPlayer`)
    (`self.K2_SetActorLocation` (`SceneComponent.GetSocketLocation` (`HSW_Hammer.MeshComp` (`self.Hammer2`)) "PlayerAttachingPoint"))))

(event `EnhancedInput|/Game/CSR/Input/Action/IA_ATTACK`
  (params (ActionValue :type Boolean) (ElapsedSeconds :type "Float (double-precision)") (TriggeredSeconds :type "Float (double-precision)") (InputAction :type "InputAction Object Reference" :default "/Game/CSR/Input/Action/IA_ATTACK.IA_ATTACK"))
  (:`Started`
    (bind (_direction _newtrack_0) (`Timeline|Timeline` :!via `PlayFromStart`)
      (:`Update`
        (`SceneComponent.K2_SetRelativeRotation` (`self.Scene`) (`KismetMathLibrary.RLerp` (`self.initRotate`) (struct :`Pitch` -180.0) _newtrack_0) false false)))))

(event `EnhancedInput|/Game/HSW/Input/Actions/IA_HSW_Hanging`
  (params (ActionValue :type Boolean) (ElapsedSeconds :type "Float (double-precision)") (TriggeredSeconds :type "Float (double-precision)") (InputAction :type "InputAction Object Reference" :default "/Game/HSW/Input/Actions/IA_HSW_Hanging.IA_HSW_Hanging"))
  (bind _hammer2 (`self.Hammer2`))
  (:`Started`
    (if (`HSW_Hammer.bCanHanging` _hammer2)
      (`HSW_Hammer.ClickToMove` _hammer2)
      (set `self.bFixPlayer` true))))

(fn `UserConstructionScript`)