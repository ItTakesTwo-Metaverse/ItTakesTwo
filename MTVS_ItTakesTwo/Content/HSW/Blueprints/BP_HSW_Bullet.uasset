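; BP_HSW_Bullet is a bullet Blueprint with a movement component and a custom event for flying back to the player.
; ReturnToPlayer runs a Timeline that lerps the bullet from its current location toward player pawn 0, without sweep, then clears the Returning flag.
; Nothing in this file calls that event or sets Returning true.
; The flag check, homing-target reset and tag-based bounce toggle are disconnected and never run.
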(event `self.ReceiveActorBeginOverlap`
  (params (OtherActor :type "Actor Object Reference")))

(event `self.ReceiveTick`
  (params (DeltaSeconds :type "Float (single-precision)")))

(event `ReturnToPlayer`
  (bind (_direction _newtrack_0) (`Timeline|Timeline`)
    (:`Update`
      (`self.K2_SetActorLocation` (`KismetMathLibrary.VLerp` (`self.K2_GetActorLocation`) (`self.K2_GetActorLocation` (`GameplayStatics.GetPlayerPawn` 0)) _newtrack_0)))
    (:`Finished`
      (set `self.bReturning` false))))

(fn `UserConstructionScript`)