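; Game mode for a two-player It Takes Two-style game, animating the May/Cody split-screen for deaths, revival and the ToolBox boss cutscene.
; Events drive timelines that lerp the cached view ratios into a custom viewport client: shrinking the dead player's view or restoring an even split.
; Death transitions end by triggering that player's heart and reborn calls.
; The cutscene expands May's view fullscreen, hides and moves her, then starts the boss's streaming cinematic.
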(event `self.ReceiveBeginPlay`
  (bind _returnvalue (`self.GetCustomViewportClient`))
  (set `self.CustomViewportClient` _returnvalue))

(event `self.MayCodyAllDieMap`)

(event `self.MayCodyAllAliveMap`
  (set `self.SaveMayview` (`CustomGameViewportClient.MayView` (`self.CustomViewportClient`)))
  (set `self.SaveCodyview` (`CustomGameViewportClient.CodyView` (`self.CustomViewportClient`)))
  (bind (_direction _mapchagetime) (`Timeline|viewChangeAlive` :!via `PlayFromStart`)
    (:`Update`
      (`CustomGameViewportClient.UpdateLayoutWithNewRatio` (`self.CustomViewportClient`) (`KismetMathLibrary.Lerp` (`self.SaveMayview`) 0.5 _mapchagetime) (`KismetMathLibrary.Lerp` (`self.SaveCodyview`) 0.5 _mapchagetime)))))

(event `self.CodyDieMap`
  (bind _p2_cody (`self.P2_Cody`))
  (set `self.SaveMayview` (`CustomGameViewportClient.MayView` (`self.CustomViewportClient`)))
  (set `self.SaveCodyview` (`CustomGameViewportClient.CodyView` (`self.CustomViewportClient`)))
  (bind (_direction _mapchagetime) (`Timeline|ViewChangeCody` :!via `PlayFromStart`)
    (:`Update`
      (`CustomGameViewportClient.UpdateLayoutWithNewRatio` (`self.CustomViewportClient`) (`KismetMathLibrary.Lerp` (`self.SaveMayview`) (`self.view66`) _mapchagetime) (`KismetMathLibrary.Lerp` (`self.SaveCodyview`) (`self.view33`) _mapchagetime)))
    (:`Finished`
      (`CSR_P_Player.ONHeart` _p2_cody)
      (`CSR_Player_Cody.tranReBorn` _p2_cody))))

(event `self.MayDieMap`
  (bind _p1_may (`self.P1_May`))
  (set `self.SaveMayview` (`CustomGameViewportClient.MayView` (`self.CustomViewportClient`)))
  (set `self.SaveCodyview` (`CustomGameViewportClient.CodyView` (`self.CustomViewportClient`)))
  (bind (_direction _mapchagetime) (`Timeline|ViewChangeMay` :!via `PlayFromStart`)
    (:`Update`
      (`CustomGameViewportClient.UpdateLayoutWithNewRatio` (`self.CustomViewportClient`) (`KismetMathLibrary.Lerp` (`self.SaveMayview`) (`self.view33`) _mapchagetime) (`KismetMathLibrary.Lerp` (`self.SaveCodyview`) (`self.view66`) _mapchagetime)))
    (:`Finished`
      (`CSR_P_Player.ONHeart` _p1_may)
      (`CSR_Player_May.tranReBorn` _p1_may))))

(event `self.CutSinMap`
  (set `self.SaveMayview` (`CustomGameViewportClient.MayView` (`self.CustomViewportClient`)))
  (set `self.SaveCodyview` (`CustomGameViewportClient.CodyView` (`self.CustomViewportClient`)))
  (bind (_direction _mapchagetime) (`Timeline|Timeline` :!via `PlayFromStart`)
    (:`Update`
      (`CustomGameViewportClient.UpdateLayoutWithNewRatio` (`self.CustomViewportClient`) (`KismetMathLibrary.Lerp` (`self.SaveMayview`) 1.0 _mapchagetime) (`KismetMathLibrary.Lerp` (`self.SaveCodyview`) 0.0 _mapchagetime)))
    (:`Finished`
      (`self.LightOn`)
      (`SceneComponent.SetVisibility` (`Character.Mesh` (`self.P1_May`)) false false)
      (`SceneComponent.SetVisibility` (`HSW_Hammer.MeshComp` (`CSR_MayUseHammerObj.Hammer` (`self.GetComponentByClass` (`self.P1_May`) "/Script/MTVS_ItTakesTwo.CSR_MayUseHammerObj"))) false false)
      (`self.K2_SetActorLocation` (`self.P1_May`) (980.0 -480.0 400.0) true false)
      (bind _asbp_tool_box_boss (cast `/Game/LHM_Boss/BluePrints/BP_ToolBoxBoss` (`self.boss`)))
      (`KismetSystemLibrary.Delay` 0.5)
      (`self.LightOff`)
      (`/Game/LHM_Boss/BluePrints/BP_ToolBoxBoss.streamingCine` _asbp_tool_box_boss))))

(event `resetVisi`
  (`SceneComponent.SetVisibility` (`Character.Mesh` (`self.P1_May`)) true false)
  (`SceneComponent.SetVisibility` (`HSW_Hammer.MeshComp` (`CSR_MayUseHammerObj.Hammer` (`self.GetComponentByClass` (`self.P1_May`) "/Script/MTVS_ItTakesTwo.CSR_MayUseHammerObj"))) true false))

(fn `NewFunction`)

(fn `UserConstructionScript`)